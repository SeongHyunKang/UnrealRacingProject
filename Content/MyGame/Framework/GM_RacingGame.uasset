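; Game mode for a timed checkpoint race, won by crossing the finish line before the countdown timer expires.
; On BeginPlay it binds to every BP_Checkpoint's finish or time-bonus dispatcher, then waits out a start delay before starting the timer.
; Checkpoints re-set the timer with remaining time plus the bonus and trigger a vehicle HUD animation.
; Start, win and lose feedback are only printed strings.
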(event Custom|Game%20Finish
  (params (Win :type Boolean))
  (Development|PrintString (Utilities|String|SelectString "You Win" "You Lose" Win)))

(event Custom|Game%20Start
  (Development|PrintString "Game Started")
  (bind _returnvalue (Utilities|Time|SetTimerbyEvent (delegate Custom|Lose_OutOfTimeCounter) (Variables|Default|GetStartTimerDuration)))
  (Variables|Default|SetTimeRemainingTimer _returnvalue))

(event Custom|Start%20Countdown
  (Development|PrintString "//Start Countdown")
  (Utilities|FlowControl|Delay (Variables|Default|GetStartCountdownDuration))
  (CallFunction|GameStart))

(event Custom|Lose_OutOfTimeCounter
  (CallFunction|GameFinish false))

(event Custom|Win_CrossedTheFinishLine
  (Utilities|Time|ClearandInvalidateTimerbyHandle (Variables|Default|GetTimeRemainingTimer))
  (CallFunction|GameFinish true))

(event Custom|CrossedCheckpoint
  (params (TimeToAdd :type Integer))
  (CallFunction|AddTimetoTimer TimeToAdd))

(event EventBeginPlay
  (Utilities|FlowControl|Sequence
    (:then_0
      (bind _outactors (Actor|GetAllActorsOfClass "/Game/MyGame/Chackpoints/BP_Checkpoint.BP_Checkpoint_C"))
      (for _array_element _outactors
        (if (Variables|/Game/MyGame/Chackpoints/BP_Checkpoint.BP_Checkpoint_C|GetisFinishLine _array_element)
          (EventDispatchers|BindEventtoOnCheckpointCrossed _array_element (EventDispatchers|CreateEvent :!event Custom|Win_CrossedTheFinishLine))
          (else
            (EventDispatchers|BindEventtoOnCheckpointCrossedwithTime _array_element (EventDispatchers|CreateEvent :!event Custom|CrossedCheckpoint))))))
    (:then_1
      (CallFunction|StartCountdown))))

(fn ConstructionScript)

(fn AddTimetoTimer
  (params (TimeToAdd :type Integer))
  (bind _returnvalue (Utilities|Time|SetTimerbyEvent (EventDispatchers|CreateEvent :!event Custom|Lose_OutOfTimeCounter) (+ (Utilities|Time|GetTimerRemainingTimebyHandle (Variables|Default|GetTimeRemainingTimer)) TimeToAdd)))
  (Variables|Default|SetTimeRemainingTimer _returnvalue)
  (bind _asvehicle_player_controller (Utilities|Casting|CastToVehiclePlayerController (Game|GetPlayerController 0)))
  (Default|PlayAnimwhenTimeAdded (Variables|/Game/VehicleTemplate/Blueprints/VehiclePlayerController.VehiclePlayerController_C|GetVehicleHud _asvehicle_player_controller)))